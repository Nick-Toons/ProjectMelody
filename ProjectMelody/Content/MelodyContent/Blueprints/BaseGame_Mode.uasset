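; Game mode for a tap-to-earn game that owns currency, upgrade and lifetime stats and persists them through MelodySave slot "save1".
; BeginPlay spawns a TouchController, forces a temporary resolution, then runs StartGameplay, which loads the save or creates one outside the main menu.
; Loading copies saved values to local variables, then CompareTime awards offline earnings from elapsed UTC time.
; EndPlay and GMSaveGame share one path that timestamps and writes an existing save.
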(event `Create Save`
  ;[1 1 1] On Game Mode play, checks if Save Game "save1" exists. If not, creates it. Calls "Set Save File To Local" to load the variables from the save file. Calls "Set Local To Save File" if no save file exists, in order to populate the file
  (bind _returnvalue (`GameplayStatics.CreateSaveGameObject` "/Game/MelodyContent/Blueprints/MelodySave.MelodySave_C"))
  (`self.Set Local To Save File`)
  (bind _returnvalue_2 (`GameplayStatics.SaveGameToSlot` _returnvalue "save1"))
  (set `self.As Melody Save` _returnvalue)
  (if _returnvalue_2
    (`KismetSystemLibrary.PrintString` "Create Save - GAME SAVED")
    (else
      (`KismetSystemLibrary.PrintString` "Create Save - SAVE FAILED" true true (struct :`R` 1.0 :`A` 1.0)))))

(event `Load Save`
  ;[1 1 1] On Game Mode play, checks if Save Game "save1" exists. If not, creates it. Calls "Set Save File To Local" to load the variables from the save file. Calls "Set Local To Save File" if no save file exists, in order to populate the file
  (bind _returnvalue (`GameplayStatics.LoadGameFromSlot` "save1" 1))
  (bind _asmelody_save (cast `/Game/MelodyContent/Blueprints/MelodySave` _returnvalue)
    (:`then`
      (set `self.As Melody Save` _asmelody_save)
      (`self.Set Save File To Local`)
      (`self.Compare Time`))
    (:`CastFailed`
      (`KismetSystemLibrary.PrintString` "WTF is a Wang Chung"))))

(event `Set Save File To Local`
  (bind _as_melody_save (`self.As Melody Save`))
  ;[1 1 1] Call this when you want to read save file variables and set them to the local variable
  (set `self.Currency` (`/Game/MelodyContent/Blueprints/MelodySave.Currency - Save` _as_melody_save))
  (set `self.Self Earned Currency Base` (`/Game/MelodyContent/Blueprints/MelodySave.Self Earned Currency Base - Save` _as_melody_save))
  (set `self.Self Earned Currency Mult` (`/Game/MelodyContent/Blueprints/MelodySave.Self Earned Currency Mult - Save` _as_melody_save))
  (set `self.Self Multiplier Increment` (`/Game/MelodyContent/Blueprints/MelodySave.Self Multiplier Increment - Save` _as_melody_save))
  (set `self.Self Upgrade 1 Cost` (`/Game/MelodyContent/Blueprints/MelodySave.Self Upgrade 1 Cost - Save` _as_melody_save))
  (set `self.Self Upgrade 1 Cost Mult` (`/Game/MelodyContent/Blueprints/MelodySave.Self Upgrade 1 Cost Mult - Save` _as_melody_save))
  (set `self.Self Upgrade 1 Count` (`/Game/MelodyContent/Blueprints/MelodySave.Self Upgrade 1 Count - Save` _as_melody_save))
  (set `self.Self Earned T Bonus` (`/Game/MelodyContent/Blueprints/MelodySave.Self Earned T Bonus - Save` _as_melody_save))
  (set `self.Self Earned T Bonus Mult` (`/Game/MelodyContent/Blueprints/MelodySave.Self Earned T Bonus Mult - Save` _as_melody_save))
  (set `self.Self Upgrade 2 Cost` (`/Game/MelodyContent/Blueprints/MelodySave.Self Upgrade 2 Cost - Save` _as_melody_save))
  (set `self.Self Upgrade 2 Cost Mult` (`/Game/MelodyContent/Blueprints/MelodySave.Self Upgrade 2 Cost Mult - Save` _as_melody_save))
  (set `self.Self Upgrade 2 Count` (`/Game/MelodyContent/Blueprints/MelodySave.Self Upgrade 2 Count - Save` _as_melody_save))
  (set `self.LifetimeEarnings` (`/Game/MelodyContent/Blueprints/MelodySave.Lifetime Currency - Save` _as_melody_save))
  (set `self.LastTime` (`/Game/MelodyContent/Blueprints/MelodySave.LastTime - Save` _as_melody_save))
  (set `self.LifetimeTaps` (`/Game/MelodyContent/Blueprints/MelodySave.Lifetime Taps - Save` _as_melody_save)))

(event `Set Local To Save File`
  (bind _as_melody_save (`self.As Melody Save`))
  ;[1 1 1] Call this when you want to write the local variables to the save file
  (set `/Game/MelodyContent/Blueprints/MelodySave.Currency - Save` (`self.Currency`) _as_melody_save)
  (set `/Game/MelodyContent/Blueprints/MelodySave.Self Earned Currency Base - Save` (`self.Self Earned Currency Base`) _as_melody_save)
  (set `/Game/MelodyContent/Blueprints/MelodySave.Self Earned Currency Mult - Save` (`self.Self Earned Currency Mult`) _as_melody_save)
  (set `/Game/MelodyContent/Blueprints/MelodySave.Self Multiplier Increment - Save` (`self.Self Multiplier Increment`) _as_melody_save)
  (set `/Game/MelodyContent/Blueprints/MelodySave.Self Upgrade 1 Cost - Save` (`self.Self Upgrade 1 Cost`) _as_melody_save)
  (set `/Game/MelodyContent/Blueprints/MelodySave.Self Upgrade 1 Cost Mult - Save` (`self.Self Upgrade 1 Cost Mult`) _as_melody_save)
  (set `/Game/MelodyContent/Blueprints/MelodySave.Self Upgrade 1 Count - Save` (`self.Self Upgrade 1 Count`) _as_melody_save)
  (set `/Game/MelodyContent/Blueprints/MelodySave.Self Earned T Bonus - Save` (`self.Self Earned T Bonus`) _as_melody_save)
  (set `/Game/MelodyContent/Blueprints/MelodySave.Self Earned T Bonus Mult - Save` (`self.Self Earned T Bonus Mult`) _as_melody_save)
  (set `/Game/MelodyContent/Blueprints/MelodySave.Self Upgrade 2 Cost - Save` (`self.Self Upgrade 2 Cost`) _as_melody_save)
  (set `/Game/MelodyContent/Blueprints/MelodySave.Self Upgrade 2 Cost Mult - Save` (`self.Self Upgrade 2 Cost Mult`) _as_melody_save)
  (set `/Game/MelodyContent/Blueprints/MelodySave.Self Upgrade 2 Count - Save` (`self.Self Upgrade 2 Count`) _as_melody_save)
  (set `/Game/MelodyContent/Blueprints/MelodySave.Lifetime Currency - Save` (`self.LifetimeEarnings`) _as_melody_save)
  (set `/Game/MelodyContent/Blueprints/MelodySave.LastTime - Save` (`self.LastTime`) _as_melody_save)
  (set `/Game/MelodyContent/Blueprints/MelodySave.Lifetime Taps - Save` (`self.LifetimeTaps`) _as_melody_save))

(event `self.ReceiveBeginPlay`
  ;[1 1 1] On Game Mode play, checks if Save Game "save1" exists. If not, creates it. Calls "Set Save File To Local" to load the variables from the save file. Calls "Set Local To Save File" if no save file exists, in order to populate the file
  (bind _returnvalue (`|SpawnActorFromClass` "/Game/MelodyContent/Blueprints/TouchController.TouchController_C" (`KismetMathLibrary.MakeTransform` (0.0 0.0 0.0)) "Undefined" "OverrideRootScale" null null))
  (bind _output_get (set `self.TouchController` _returnvalue))
  (set `PlayerController.bShowMouseCursor` true _output_get)
  (`KismetSystemLibrary.ExecuteConsoleCommand` "r.SetRes 608x1280" null) ; Temporary node to force the resolution we have currently set in our UI BPs
  (`self.Start Gameplay`))

(event `Start Gameplay`
  ;[1 1 1] On Game Mode play, checks if Save Game "save1" exists. If not, creates it. Calls "Set Save File To Local" to load the variables from the save file. Calls "Set Local To Save File" if no save file exists, in order to populate the file
  ;;[1 1 1] Custom command for "Event BeginPlay" and MainMenuTest's "Start Game" button to run to ensure that a Save File isn't generated immediately on game load, but rather when the user WANTS to start the game
  (set `self.LastTime` (`KismetMathLibrary.UtcNow`))
  (bind _returnvalue (`GameplayStatics.DoesSaveGameExist` "save1"))
  (if _returnvalue
    (`self.Load Save`)
    (else
      (bind _returnvalue_2 (`GameplayStatics.GetCurrentLevelName` true))
      (if (not (`KismetStringLibrary.EqualEqual_StrStr` _returnvalue_2 (`self.MainMenuName`)))
        (`self.Create Save`)))))

(event `self.ReceiveEndPlay`
  (params (EndPlayReason :type "EEndPlayReason Enum" :default "Destroyed"))
  (bind _returnvalue (`KismetStringLibrary.Concat_StrStr` "Exit/Save Currency: " (`KismetStringLibrary.Conv_DoubleToString` (`self.Currency`))))
  ;[1 1 1] When closing the game, or hitting any of the save buttons, calls either End Play, or the custom GM Save Game commands, to manually save all the needed variables.
  (bind _returnvalue_2 (`GameplayStatics.DoesSaveGameExist` "save1" :!label _label))
  (if _returnvalue_2
    (set `self.LastTime` (`KismetMathLibrary.UtcNow`))
    (`self.Set Local To Save File`)
    (bind _returnvalue_3 (`GameplayStatics.SaveGameToSlot` (`self.As Melody Save`) "save1"))
    (if _returnvalue_3
      (`KismetSystemLibrary.PrintString` "Exit/Save - GAME SAVED")
      (`KismetSystemLibrary.PrintString` _returnvalue true true (struct :`G` 0.011288 :`B` 1.0 :`A` 1.0))
      (else
        (`KismetSystemLibrary.PrintString` "Exit/Save - SAVE FAILED" true true (struct :`R` 1.0 :`A` 1.0))
        (`KismetSystemLibrary.PrintString` _returnvalue true true (struct :`G` 0.039349 :`B` 1.0 :`A` 1.0))))))

(event `GM Save Game`
  ;[1 1 1] When closing the game, or hitting any of the save buttons, calls either End Play, or the custom GM Save Game commands, to manually save all the needed variables.
  (goto _label))

(event `Compare Time`
  (bind (_days _hours _minutes _seconds _milliseconds) (`KismetMathLibrary.BreakTimespan` (- (`KismetMathLibrary.UtcNow`) (`self.LastTime`))))
  (bind _returnvalue (* (* (+ (* _days 86400) (* _hours 3600) (* _minutes 60) _seconds (/ _milliseconds 1000)) (`self.Timeout Multiplier`)) (* (`self.Self Earned Currency Base`) (`self.Self Earned Currency Mult`))))
  ;[1 1 1] Takes current time of the device upon boot, and compares it to what timestamp is on the save file. Awards player "AFK Currency" and adds it to their loadout at a smaller rate
  (`KismetSystemLibrary.PrintString` (`KismetStringLibrary.Concat_StrStr` "Time Boost: " (`KismetStringLibrary.Conv_DoubleToString` _returnvalue)) true true (struct :`R` 0.050572 :`G` 1.0 :`A` 1.0))
  (set `self.Currency` (`KismetMathLibrary.Conv_IntToDouble` (`KismetMathLibrary.FTrunc` (+ _returnvalue (`self.Currency`)))))
  (set `self.LifetimeEarnings` (`KismetMathLibrary.Conv_IntToDouble` (`KismetMathLibrary.FTrunc` (+ (`self.LifetimeEarnings`) _returnvalue)))))

(fn `UserConstructionScript`)