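; Blueprint function library for the game, with a Set String function that turns a numeric note value into shorthand display text.
; A descending branch chain picks trillion, billion, million or thousand, divides by that scale, formats the float as text and appends T, B, M or K.
; Values below a thousand are truncated to a whole number without a suffix, and the caller decides how the returned string is used.
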(fn `Set String`
  (params (`Note Value` :type "Float (double-precision)"))
  (returns (`Output String` :type String))
  ;[1 1 1] Function created to take an input value, and output it in a shorthand string form. What you do with the string output is up to you
  (if (>= `Note Value` 999999995904.0)
    (return (`KismetStringLibrary.Concat_StrStr` (`KismetTextLibrary.Conv_TextToString` (`KismetTextLibrary.Conv_DoubleToText` (/ `Note Value` 999999995904.0) "HalfToEven" false true 1 324 3)) "T"))
    (elif (>= `Note Value` 1000000000.0)
      (return (`KismetStringLibrary.Concat_StrStr` (`KismetTextLibrary.Conv_TextToString` (`KismetTextLibrary.Conv_DoubleToText` (/ `Note Value` 1000000000.0) "HalfToEven" false true 1 324 3)) "B"))
      (elif (>= `Note Value` 1000000.0)
        (return (`KismetStringLibrary.Concat_StrStr` (`KismetTextLibrary.Conv_TextToString` (`KismetTextLibrary.Conv_DoubleToText` (/ `Note Value` 1000000.0) "HalfToEven" false true 1 324 3)) "M"))
        (elif (>= `Note Value` 1000.0)
          (return (`KismetStringLibrary.Concat_StrStr` (`KismetTextLibrary.Conv_TextToString` (`KismetTextLibrary.Conv_DoubleToText` (/ `Note Value` 1000.0) "HalfToEven" false true 1 324 3)) "K"))
          (else
            (return (`KismetStringLibrary.Conv_IntToString` (`KismetMathLibrary.FTrunc` `Note Value`)))))))))